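; MazeWall is a wall actor, apparently for a maze, built from a spline mesh spanning a start and end location.
; The construction script sets the mesh's end position along local X to the distance between the two points.
; It rotates the actor to look from start to end, so the wall stays straight, then makes the mesh static.
; The event graph holds only disabled placeholder events.
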(fn `UserConstructionScript`
  (`SplineMeshComponent.SetEndPosition` (`self.SplineMesh`) (`KismetMathLibrary.MakeVector` (`KismetMathLibrary.Vector_Distance` (`self.StartLocation`) (`self.EndLocation`))) true)
  (`self.K2_SetActorRotation` (`KismetMathLibrary.FindLookAtRotation` (`self.StartLocation`) (`self.EndLocation`)))
  (`SceneComponent.SetMobility` (`self.SplineMesh`) "Static"))