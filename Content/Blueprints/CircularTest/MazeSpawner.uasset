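; Actor that generates a random circular maze on BeginPlay from concentric rings split into sectors.
; It builds Segment objects keyed "Sector-Level", then random-walks a path from the outer ring to the center.
; Outer and inner boundaries get random openings, then path sides and remaining segments get walls, denser near the center.
; CreateWall spawns attached MazeWall actors and updates neighboring segments, and DrawPath debug-draws the route.
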(event `self.ReceiveBeginPlay`
  (`self.CreateSegments`)
  (`self.GeneratePath`)
  (`self.GenerateOuterWall`)
  (`self.GenerateInnerWall`)
  (`self.GeneratePathWall`)
  (`self.GenerateRemainingWall`)
  (`self.DrawPath`))

(fn `ClampSectorNumber`
  (params (NewSectorName :type Integer))
  (returns (SectorNumber :type Integer))
  (if (> NewSectorName 0)
    (return (+ (mod (- NewSectorName 1) (`self.Sectors`)) 1))
    (else
      (return (+ (`self.Sectors`) NewSectorName)))))

(fn `CreateSegments`
  (locals (CurrentSector :type Integer))
  (for _index (range 1 (+ (`self.Sectors`) 1))
    (set `local.CurrentSector` _index)
    (for _index_2 (range 1 (+ (`self.Levels`) 1))
      (bind _returnvalue (`KismetStringLibrary.Concat_StrStr` (`KismetStringLibrary.Conv_IntToString` (`local.CurrentSector`)) "-" (`KismetStringLibrary.Conv_IntToString` _index_2)))
      (bind _returnvalue_2 (`|GenericCreateObject` self "/Game/Blueprints/CircularTest/Segment.Segment_C" _returnvalue self))
      (`BlueprintMapLibrary.Map_Add` (`self.Segments`) _returnvalue _returnvalue_2)
      (`/Game/Blueprints/CircularTest/Segment.Init` _returnvalue_2 (`self.GetActorForwardVector`) (`self.Sectors`) (`self.InnerRadius`) (`self.LevelDistance`)))))

(fn `CreateWall`
  (params (Segment :type String) (WallType :type "/Game/Blueprints/CircularTest/EnumType/WallType Enum" :default "NewEnumerator0") (OuterWallofMaze :type Boolean) (InnerWallofMaze :type Boolean))
  (returns (Result :type Boolean))
  (locals (BorderingSegment :type String))
  (bind (_segmentexists _borderingsegment) (`self.GetBorderingSegment` Segment WallType))
  (bind _value (`BlueprintMapLibrary.Map_Find` (`self.Segments`) Segment))
  (bind _value_2 (`BlueprintMapLibrary.Map_Find` (`self.Segments`) Segment))
  (bind _value_3 (`BlueprintMapLibrary.Map_Find` (`self.Segments`) Segment))
  (bind _value_4 (`BlueprintMapLibrary.Map_Find` (`self.Segments`) Segment))
  (bind _value_5 (`BlueprintMapLibrary.Map_Find` (`self.Segments`) Segment))
  (bind _value_6 (`BlueprintMapLibrary.Map_Find` (`self.Segments`) Segment))
  (bind _cornerlocation (`/Game/Blueprints/CircularTest/Segment.CornerLocation` _value_4))
  (bind _cornerlocation_2 (`/Game/Blueprints/CircularTest/Segment.CornerLocation` _value_5))
  (bind _cornerlocation_3 (`/Game/Blueprints/CircularTest/Segment.CornerLocation` _value_6))
  (bind _cornerlocation_4 (`/Game/Blueprints/CircularTest/Segment.CornerLocation` _value))
  (bind _cornerlocation_5 (`/Game/Blueprints/CircularTest/Segment.CornerLocation` _value_2))
  (bind _cornerlocation_6 (`/Game/Blueprints/CircularTest/Segment.CornerLocation` _value_3))
  (bind _value_7 (`BlueprintMapLibrary.Map_Find` _cornerlocation_4 "NewEnumerator0"))
  (bind _value_8 (`BlueprintMapLibrary.Map_Find` _cornerlocation_5 "NewEnumerator1"))
  (bind _value_9 (`BlueprintMapLibrary.Map_Find` _cornerlocation_6 "NewEnumerator3"))
  (bind _value_10 (`BlueprintMapLibrary.Map_Find` _cornerlocation "NewEnumerator0"))
  (bind _value_11 (`BlueprintMapLibrary.Map_Find` _cornerlocation_2 "NewEnumerator1"))
  (bind _value_12 (`BlueprintMapLibrary.Map_Find` _cornerlocation_3 "NewEnumerator1"))
  (if OuterWallofMaze
    ;[1 1 1] Comment
    (`/Game/Blueprints/CircularTest/Segment.AddWall` _value "NewEnumerator0")
    (bind _returnvalue (`|SpawnActorFromClass` "/Game/Blueprints/CircularTest/MazeWall.MazeWall_C" (`KismetMathLibrary.MakeTransform` _value_7) "Undefined" "OverrideRootScale" null _value_7 (`BlueprintMapLibrary.Map_Find` _cornerlocation_4 "NewEnumerator2") null))
    (`self.K2_AttachToActor` _returnvalue self "None" "KeepWorld" "KeepWorld" "KeepWorld" true)
    (return true)
    (elif (and (`|EnumEquality` WallType "NewEnumerator0") (== (`.RightS` (`KismetStringLibrary.Split` Segment "-")) (`self.Levels`)))
      (return false)
      (elif InnerWallofMaze
        ;[1 1 1] Comment
        (`/Game/Blueprints/CircularTest/Segment.AddWall` _value_2 "NewEnumerator1")
        (bind _returnvalue_2 (`|SpawnActorFromClass` "/Game/Blueprints/CircularTest/MazeWall.MazeWall_C" (`KismetMathLibrary.MakeTransform` _value_8) "Undefined" "OverrideRootScale" null _value_8 (`BlueprintMapLibrary.Map_Find` _cornerlocation_5 "NewEnumerator3") null))
        (`self.K2_AttachToActor` _returnvalue_2 self "None" "KeepWorld" "KeepWorld" "KeepWorld" true)
        (return true)
        (elif (and (`|EnumEquality` WallType "NewEnumerator1") (== (`.RightS` (`KismetStringLibrary.Split` Segment "-")) 1))
          (return false)
          (elif _segmentexists
            (set `local.BorderingSegment` _borderingsegment)
            (switch `/Game/Blueprints/CircularTest/EnumType/WallType` WallType
              (:`NewEnumerator0`
                ;[1 1 1] Comment
                (`/Game/Blueprints/CircularTest/Segment.AddWall` _value_4 "NewEnumerator0")
                (bind _returnvalue_3 (`|SpawnActorFromClass` "/Game/Blueprints/CircularTest/MazeWall.MazeWall_C" (`KismetMathLibrary.MakeTransform` _value_10) "Undefined" "OverrideRootScale" null _value_10 (`BlueprintMapLibrary.Map_Find` _cornerlocation "NewEnumerator2") null))
                (`self.K2_AttachToActor` _returnvalue_3 self "None" "KeepWorld" "KeepWorld" "KeepWorld" true)
                (`/Game/Blueprints/CircularTest/Segment.AddWall` (`BlueprintMapLibrary.Map_Find` (`self.Segments`) (`local.BorderingSegment`)) "NewEnumerator1")
                (return true))
              (:`NewEnumerator1`
                ;[1 1 1] Comment
                (`/Game/Blueprints/CircularTest/Segment.AddWall` _value_5 "NewEnumerator1")
                (bind _returnvalue_4 (`|SpawnActorFromClass` "/Game/Blueprints/CircularTest/MazeWall.MazeWall_C" (`KismetMathLibrary.MakeTransform` _value_11) "Undefined" "OverrideRootScale" null _value_11 (`BlueprintMapLibrary.Map_Find` _cornerlocation_2 "NewEnumerator3") null))
                (`self.K2_AttachToActor` _returnvalue_4 self "None" "KeepWorld" "KeepWorld" "KeepWorld" true)
                (`/Game/Blueprints/CircularTest/Segment.AddWall` (`BlueprintMapLibrary.Map_Find` (`self.Segments`) (`local.BorderingSegment`)) "NewEnumerator0")
                (return true))
              (:`NewEnumerator2`
                ;[1 1 1] Comment
                (`/Game/Blueprints/CircularTest/Segment.AddWall` _value_6 "NewEnumerator2")
                (bind _returnvalue_5 (`|SpawnActorFromClass` "/Game/Blueprints/CircularTest/MazeWall.MazeWall_C" (`KismetMathLibrary.MakeTransform` _value_12) "Undefined" "OverrideRootScale" null _value_12 (`BlueprintMapLibrary.Map_Find` _cornerlocation_3 "NewEnumerator0") null))
                (`self.K2_AttachToActor` _returnvalue_5 self "None" "KeepWorld" "KeepWorld" "KeepWorld" true)
                (`/Game/Blueprints/CircularTest/Segment.AddWall` (`BlueprintMapLibrary.Map_Find` (`self.Segments`) (`local.BorderingSegment`)) "NewEnumerator3")
                (return true))
              (:`NewEnumerator3`
                ;[1 1 1] Comment
                (`/Game/Blueprints/CircularTest/Segment.AddWall` _value_3 "NewEnumerator3")
                (bind _returnvalue_6 (`|SpawnActorFromClass` "/Game/Blueprints/CircularTest/MazeWall.MazeWall_C" (`KismetMathLibrary.MakeTransform` _value_9) "Undefined" "OverrideRootScale" null _value_9 (`BlueprintMapLibrary.Map_Find` _cornerlocation_6 "NewEnumerator2") null))
                (`self.K2_AttachToActor` _returnvalue_6 self "None" "KeepWorld" "KeepWorld" "KeepWorld" true)
                (`/Game/Blueprints/CircularTest/Segment.AddWall` (`BlueprintMapLibrary.Map_Find` (`self.Segments`) (`local.BorderingSegment`)) "NewEnumerator2")
                (return true)))
            (else
              (return false))))))))

(fn `DrawPath`
  (locals (PreviousSegment :type String))
  (set `local.PreviousSegment` (`|GetArrayItem` (`self.Path`) 1))
  (for _array_element (`self.Path`)
    (if (`BlueprintMapLibrary.Map_Contains` (`self.Segments`) _array_element)
      (`KismetSystemLibrary.DrawDebugLine` (`/Game/Blueprints/CircularTest/Segment.GetCenter` (`BlueprintMapLibrary.Map_Find` (`self.Segments`) (`local.PreviousSegment`))) (`/Game/Blueprints/CircularTest/Segment.GetCenter` (`BlueprintMapLibrary.Map_Find` (`self.Segments`) _array_element)) (struct :`A` 1.0) 30.0 25.0)
      (set `local.PreviousSegment` _array_element))))

(fn `GenerateInnerWall`
  (locals (MaxExits :type Integer) (PathExitSegment :type Integer) (AvailableSegment :type "Array of String") (CurrentExit :type String))
  (bind _path (`self.Path`))
  (bind _availablesegment (`local.AvailableSegment`))
  (bind _availablesegment_2 (`local.AvailableSegment`))
  (bind _currentexit (`local.CurrentExit`))
  (bind _lefts (`KismetStringLibrary.Split` _currentexit "-"))
  (bind _returnvalue (`KismetStringLibrary.Concat_StrStr` (`KismetStringLibrary.Conv_IntToString` (`self.ClampSectorNumber` (+ _lefts 1))) "-" "1"))
  (bind _returnvalue_2 (`KismetStringLibrary.Concat_StrStr` (`KismetStringLibrary.Conv_IntToString` (`self.ClampSectorNumber` (- _lefts 1))) "-" "1"))
  ;[1 1 1] Comment
  (set `local.MaxExits` (/ (`self.Sectors`) 7))
  (set `local.PathExitSegment` (`KismetStringLibrary.Conv_StringToInt` (`KismetStringLibrary.Split` (`|GetArrayItem` _path (`KismetArrayLibrary.Array_LastIndex` _path)) "-")))
  (for _index (range 1 (+ (`self.Sectors`) 1))
    ;[1 1 1] Comment
    (if (> (`KismetMathLibrary.Abs_Int` (- _index (`local.PathExitSegment`))) 1)
      ;[1 1 1] Comment
      (`KismetArrayLibrary.Array_Add` (`local.AvailableSegment`) (`KismetStringLibrary.Concat_StrStr` (`KismetStringLibrary.Conv_IntToString` _index) "-" "1"))
      (else
        ;[1 1 1] Comment
        (if (!= _index (`local.PathExitSegment`))
          (`self.CreateWall` (`KismetStringLibrary.Concat_StrStr` (`KismetStringLibrary.Conv_IntToString` _index) "-" "1") "NewEnumerator1" false true)))))
  (for _ (range 1 (+ (`local.MaxExits`) 1))
    ;[1 1 1] Comment
    (bind _output_get (set `local.CurrentExit` (`self.GetRandomArrayElement` _availablesegment_2)))
    (`KismetArrayLibrary.Array_Add` (`self.Exits`) _output_get)
    (`KismetArrayLibrary.Array_RemoveItem` _availablesegment_2 _currentexit)
    ;[1 1 1] Comment
    (`self.CreateWall` _returnvalue "NewEnumerator1" false true)
    (`KismetArrayLibrary.Array_RemoveItem` _availablesegment _returnvalue)
    (`self.CreateWall` _returnvalue_2 "NewEnumerator1" false true)
    (`KismetArrayLibrary.Array_RemoveItem` _availablesegment _returnvalue_2))
  ;[1 1 1] Comment
  (for _array_element (`local.AvailableSegment`)
    (`self.CreateWall` _array_element "NewEnumerator1" false true)))

(fn `GenerateOuterWall`
  (locals (MaxEntrances :type Integer) (PathEntranceSegment :type Integer) (AvailableSegment :type "Array of String") (CurrentEntrance :type String))
  (bind _currententrance (`local.CurrentEntrance`))
  (bind _availablesegment (`local.AvailableSegment`))
  (bind _availablesegment_2 (`local.AvailableSegment`))
  (bind (_lefts _rights) (`KismetStringLibrary.Split` _currententrance "-"))
  (bind _returnvalue (`KismetStringLibrary.Concat_StrStr` (`KismetStringLibrary.Conv_IntToString` (`self.ClampSectorNumber` (+ _lefts 1))) "-" _rights))
  (bind _returnvalue_2 (`KismetStringLibrary.Concat_StrStr` (`KismetStringLibrary.Conv_IntToString` (`self.ClampSectorNumber` (+ _lefts 1))) "-" _rights))
  (set `local.MaxEntrances` (/ (`self.Sectors`) 5))
  (set `local.PathEntranceSegment` (`KismetStringLibrary.Conv_StringToInt` (`KismetStringLibrary.Split` (`|GetArrayItem` (`self.Path`)) "-")))
  (for _index (range 1 (+ (`self.Sectors`) 1))
    ;[1 1 1] Comment
    (if (> (`KismetMathLibrary.Abs_Int` (- _index (`local.PathEntranceSegment`))) 0)
      ;[1 1 1] Comment
      (`KismetArrayLibrary.Array_Add` (`local.AvailableSegment`) (`KismetStringLibrary.Concat_StrStr` (`KismetStringLibrary.Conv_IntToString` _index) "-" (`KismetStringLibrary.Conv_IntToString` (`self.Levels`))))
      (else
        ;[1 1 1] Comment
        (if (!= _index (`local.PathEntranceSegment`))
          (`self.CreateWall` (`KismetStringLibrary.Concat_StrStr` (`KismetStringLibrary.Conv_IntToString` _index) "-" (`KismetStringLibrary.Conv_IntToString` (`self.Levels`))) "NewEnumerator0" true)))))
  (for _ (range 1 (+ (`local.MaxEntrances`) 1))
    ;[1 1 1] Comment
    (bind _output_get (set `local.CurrentEntrance` (`self.GetRandomArrayElement` _availablesegment_2)))
    (`KismetArrayLibrary.Array_Add` (`self.Entrances`) _output_get)
    (`KismetArrayLibrary.Array_RemoveItem` _availablesegment_2 _currententrance)
    ;[1 1 1] Comment
    (`self.CreateWall` _returnvalue "NewEnumerator0" true)
    (`KismetArrayLibrary.Array_RemoveItem` _availablesegment _returnvalue)
    (`self.CreateWall` _returnvalue_2 "NewEnumerator0" true)
    (`KismetArrayLibrary.Array_RemoveItem` _availablesegment _returnvalue_2))
  ;[1 1 1] Comment
  (for _array_element (`local.AvailableSegment`)
    (`self.CreateWall` _array_element "NewEnumerator0" true)))

(fn `GeneratePath`
  (locals (PathLateralChance :type "Float (double-precision)" :default 0.65) (NumLateralSectors :type Integer) (CurrentSector :type Integer) (CurrentLevel :type Integer) (MaxLateralsOnLevel :type Integer :default 4) (GoClockwise :type Boolean))
  (set `local.CurrentLevel` (`self.Levels`))
  (set `local.CurrentSector` (`KismetMathLibrary.RandomIntegerInRange` 1 (`self.Sectors`)))
  (`KismetArrayLibrary.Array_Add` (`self.Path`) (`KismetStringLibrary.Concat_StrStr` (`KismetStringLibrary.Conv_IntToString` (`local.CurrentSector`)) "-" (`KismetStringLibrary.Conv_IntToString` (`local.CurrentLevel`))))
  (while (not (`self.PathReachedCenter`))
    (if (< (`local.NumLateralSectors`) 1)
      ;[1 1 1] Go Laterally
      (set `local.GoClockwise` (`KismetMathLibrary.RandomBool`) :!label _label)
      (set `local.CurrentSector` (`self.ClampSectorNumber` (+ (`local.CurrentSector`) (select `bool` (`local.GoClockwise`) :`false` -1 :`true` 1))))
      (if (`KismetArrayLibrary.Array_Contains` (`self.Path`) (`KismetStringLibrary.Concat_StrStr` (`KismetStringLibrary.Conv_IntToString` (`local.CurrentSector`)) "-" (`KismetStringLibrary.Conv_IntToString` (`local.CurrentLevel`))))
        (set `local.CurrentSector` (`self.ClampSectorNumber` (+ (`local.CurrentSector`) (select `bool` (`local.GoClockwise`) :`false` 2 :`true` -2)))))
      ;;[1 1 1] Comment
      (`KismetArrayLibrary.Array_Add` (`self.Path`) (`KismetStringLibrary.Concat_StrStr` (`KismetStringLibrary.Conv_IntToString` (`local.CurrentSector`)) "-" (`KismetStringLibrary.Conv_IntToString` (`local.CurrentLevel`))))
      (`/Engine/EditorBlueprintResources/StandardMacros.IncrementInt` (`local.NumLateralSectors`))
      (else
        ;[1 1 1] Comment
        (if (and (<= (`KismetMathLibrary.RandomFloat`) (`local.PathLateralChance`)) (< (`local.NumLateralSectors`) (`local.MaxLateralsOnLevel`)))
          (goto _label)
          (else
            ;[1 1 1] Comment
            (`/Engine/EditorBlueprintResources/StandardMacros.DecrementInt` (`local.CurrentLevel`)
              (:`  `
                (`KismetArrayLibrary.Array_Add` (`self.Path`) (`KismetStringLibrary.Concat_StrStr` (`KismetStringLibrary.Conv_IntToString` (`local.CurrentSector`)) "-" (`KismetStringLibrary.Conv_IntToString` (`local.CurrentLevel`))))
                (set `local.NumLateralSectors` 0)))))))))

(fn `GeneratePathWall`
  (locals (WallsInARow :type Integer) (AvailableWall :type "Array of /Game/Blueprints/CircularTest/EnumType/WallType Enum") (CurrentSegment :type String))
  (for _array_element (`self.Path`)
    (bind _output_get (set `local.CurrentSegment` _array_element))
    ;[1 1 1] Comment
    (if (!= (`.RightS` (`KismetStringLibrary.Split` _output_get "-")) "0")
      ;[1 1 1] Comment
      (bind _output_get_2 (set `local.AvailableWall` (`/Game/Blueprints/CircularTest/Segment.GetAvailableWall` (`BlueprintMapLibrary.Map_Find` (`self.Segments`) (`local.CurrentSegment`)))))
      ;[1 1 1] Comment
      (`KismetArrayLibrary.Array_Shuffle` (`local.AvailableWall`))
      (for _array_element_2 _output_get_2
        (bind (_segmentexists _borderingsegment) (`self.GetBorderingSegment` (`local.CurrentSegment`) _array_element_2))
        (if _segmentexists
          ;[1 1 1] Comment
          (if (not (`KismetArrayLibrary.Array_Contains` (`self.Path`) _borderingsegment))
            ;[1 1 1] Comment
            (if (>= (`local.WallsInARow`) 3)
              ;[1 1 1] Comment
              (set `local.WallsInARow` 0)
              (else
                ;[1 1 1] Comment
                (bind _result (`self.CreateWall` (`local.CurrentSegment`) _array_element_2))
                (if _result
                  (`/Engine/EditorBlueprintResources/StandardMacros.IncrementInt` (`local.WallsInARow`)))))))))))

(fn `GenerateRemainingWall`
  (locals (AvailableSector :type "Array of String") (AvailableWall :type "Array of /Game/Blueprints/CircularTest/EnumType/WallType Enum") (CurrentSegment :type String) (BorderingSegment :type String))
  (bind _value (`BlueprintMapLibrary.Map_Find` (`self.Segments`) (`local.BorderingSegment`)))
  (bind _value_2 (`BlueprintMapLibrary.Map_Find` (`self.Segments`) (`local.CurrentSegment`)))
  (bind _keys (`BlueprintMapLibrary.Map_Keys` (`self.Segments`)))
  (set `local.AvailableSector` _keys)
  ;[1 1 1] Comment
  (for _array_element (`self.Path`)
    (`KismetArrayLibrary.Array_RemoveItem` (`local.AvailableSector`) _array_element))
  ;[1 1 1] Comment
  (for _array_element_2 (`self.Entrances`)
    (`KismetArrayLibrary.Array_RemoveItem` (`local.AvailableSector`) _array_element_2))
  ;[1 1 1] Comment
  (for _array_element_3 (`self.Exits`)
    (`KismetArrayLibrary.Array_RemoveItem` (`local.AvailableSector`) _array_element_3))
  (for _array_element_4 (`local.AvailableSector`)
    (set `local.CurrentSegment` _array_element_4)
    ;[1 1 1] Comment
    (bind _output_get (set `local.AvailableWall` (`/Game/Blueprints/CircularTest/Segment.GetAvailableWall` (`BlueprintMapLibrary.Map_Find` (`self.Segments`) (`local.CurrentSegment`)))))
    (for _array_element_5 _output_get
      (bind (_segmentexists _borderingsegment) (`self.GetBorderingSegment` (`local.CurrentSegment`) _array_element_5))
      (if _segmentexists
        (set `local.BorderingSegment` _borderingsegment)
        ;[1 1 1] Comment
        (if (not (`KismetArrayLibrary.Array_Contains` (`self.Entrances`) (`local.BorderingSegment`)))
          ;[1 1 1] Comment
          (if (not (`KismetArrayLibrary.Array_Contains` (`self.Exits`) (`local.BorderingSegment`)))
            (`/Engine/EditorBlueprintResources/StandardMacros.IsValid` _value
              (:`Is Valid`
                (`/Engine/EditorBlueprintResources/StandardMacros.IsValid` _value_2
                  (:`Is Valid`
                    ;[1 1 1] Comment
                    (if (and (> (`KismetArrayLibrary.Array_Length` (`/Game/Blueprints/CircularTest/Segment.GetAvailableWall` _value)) 1) (> (`KismetArrayLibrary.Array_Length` (`/Game/Blueprints/CircularTest/Segment.GetAvailableWall` _value_2)) 1))
                      ;[1 1 1] Comment
                      (if (<= (`KismetMathLibrary.RandomFloat`) (+ (`self.WallFrequency`) (* (`KismetMathLibrary.Clamp` (- 5 (`.RightS` (`KismetStringLibrary.Split` (`local.CurrentSegment`) "-"))) 0 1999999) 0.025)))
                        ;[1 1 1] Comment
                        (`self.CreateWall` (`local.CurrentSegment`) _array_element_5)))))))))))))

(fn `GetBorderingSegment`
  (params (Segment :type String) (Border :type "/Game/Blueprints/CircularTest/EnumType/WallType Enum" :default "NewEnumerator0"))
  (returns (SegmentExists :type Boolean) (BorderingSegment :type String))
  (locals (Sector :type Integer) (Level :type Integer))
  (bind (_lefts _rights) (`KismetStringLibrary.Split` Segment "-"))
  (bind _returnvalue (`KismetStringLibrary.Concat_StrStr` (`KismetStringLibrary.Conv_IntToString` (`local.Sector`)) "-" (`KismetStringLibrary.Conv_IntToString` (`local.Level`))))
  (set `local.Sector` (`KismetStringLibrary.Conv_StringToInt` _lefts))
  (set `local.Level` (`KismetStringLibrary.Conv_StringToInt` _rights))
  (switch `/Game/Blueprints/CircularTest/EnumType/WallType` Border
    (:`NewEnumerator0`
      ;[1 1 1] Comment
      (bind _result (`/Engine/EditorBlueprintResources/StandardMacros.IncrementInt` (`local.Level`))
        (:`  `
          (if (> _result (`self.Levels`))
            (return false "")
            (else
              (return true _returnvalue))))))
    (:`NewEnumerator1`
      ;[1 1 1] Comment
      (bind _result_2 (`/Engine/EditorBlueprintResources/StandardMacros.DecrementInt` (`local.Level`))
        (:`  `
          (if (== _result_2 (`self.Levels`))
            (return false "")
            (else
              (return true _returnvalue))))))
    (:`NewEnumerator2`
      ;[1 1 1] Comment
      (set `local.Sector` (`self.ClampSectorNumber` (- (`local.Sector`) 1)))
      (return true _returnvalue))
    (:`NewEnumerator3`
      ;[1 1 1] Comment
      (set `local.Sector` (`self.ClampSectorNumber` (+ (`local.Sector`) 1)))
      (return true _returnvalue))))

(fn `PathReachedCenter`
  (returns (Result :type Boolean))
  (bind _path (`self.Path`))
  (return (== (`.RightS` (`KismetStringLibrary.Split` (`|GetArrayItem` _path (`KismetArrayLibrary.Array_LastIndex` _path)) "-")) "0")))

(fn `UserConstructionScript`)