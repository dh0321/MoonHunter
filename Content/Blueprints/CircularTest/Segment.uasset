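; Segment represents one cell of a circular maze, tracking its walls and world-space corners.
; Init parses sector and ring level from its hyphenated name, then computes four corners by rotating a forward vector around Z and scaling by ring radius.
; A wall map records which wall types exist and reports those still absent.
; Its center is the midpoint of two diagonal corners.
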(fn `AddWall`
  (params (WallType :type "/Game/Blueprints/CircularTest/EnumType/WallType Enum" :default "NewEnumerator0"))
  (`BlueprintMapLibrary.Map_Add` (`self.Walls`) WallType true)
  (return))

(fn `CalculateCornerLocation`
  (params (ForwardVector :type "Vector Structure") (NumSectors :type Integer) (InnerRadius :type "Float (double-precision)") (RingDistance :type "Float (double-precision)"))
  (locals (SectorAngle :type "Float (double-precision)"))
  (set `local.SectorAngle` (`KismetMathLibrary.Conv_IntToDouble` (/ 360 NumSectors)))
  (`BlueprintMapLibrary.Map_Add` (`self.CornerLocation`) "NewEnumerator1" (+ (* (`KismetMathLibrary.RotateAngleAxis` ForwardVector (* (- (`self.Sector`) 1) (`local.SectorAngle`)) (0.0 0.0 1.0)) (+ (* (- (`self.Level`) 1) RingDistance) InnerRadius)) (`self.MazeCenter`)))
  (`BlueprintMapLibrary.Map_Add` (`self.CornerLocation`) "NewEnumerator3" (+ (* (`KismetMathLibrary.RotateAngleAxis` ForwardVector (* (`self.Sector`) (`local.SectorAngle`)) (0.0 0.0 1.0)) (+ (* (- (`self.Level`) 1) RingDistance) InnerRadius)) (`self.MazeCenter`)))
  (`BlueprintMapLibrary.Map_Add` (`self.CornerLocation`) "NewEnumerator0" (+ (* (`KismetMathLibrary.RotateAngleAxis` ForwardVector (* (- (`self.Sector`) 1) (`local.SectorAngle`)) (0.0 0.0 1.0)) (+ (* (`self.Level`) RingDistance) InnerRadius)) (`self.MazeCenter`)))
  (`BlueprintMapLibrary.Map_Add` (`self.CornerLocation`) "NewEnumerator2" (+ (* (`KismetMathLibrary.RotateAngleAxis` ForwardVector (* (`self.Sector`) (`local.SectorAngle`)) (0.0 0.0 1.0)) (+ (* (`self.Level`) RingDistance) InnerRadius)) (`self.MazeCenter`)))
  (return))

(fn `DoesWallExist`
  (params (WallType :type "/Game/Blueprints/CircularTest/EnumType/WallType Enum" :default "NewEnumerator0"))
  (returns (Result :type Boolean))
  (return (`BlueprintMapLibrary.Map_Find` (`self.Walls`) WallType)))

(fn `GetAvailableWall`
  (returns (AvailableWalls :type "Array of /Game/Blueprints/CircularTest/EnumType/WallType Enum"))
  (locals (LocalAvailableWalls :type "Array of /Game/Blueprints/CircularTest/EnumType/WallType Enum"))
  (bind _keys (`BlueprintMapLibrary.Map_Keys` (`self.Walls`)))
  (for _array_element _keys
    (if (not (`self.DoesWallExist` _array_element))
      (`KismetArrayLibrary.Array_Add` (`local.LocalAvailableWalls`) _array_element)))
  (return (`local.LocalAvailableWalls`)))

(fn `GetCenter`
  (returns (Center :type "Vector Structure"))
  (return (/ (+ (`BlueprintMapLibrary.Map_Find` (`self.CornerLocation`) "NewEnumerator0") (`BlueprintMapLibrary.Map_Find` (`self.CornerLocation`) "NewEnumerator3")) 2.0)))

(fn `Init`
  (params (ForwardVector :type "Vector Structure") (NumSector :type Integer) (InnerRadius :type "Float (double-precision)") (RingDistance :type "Float (double-precision)"))
  (bind (_lefts _rights) (`KismetStringLibrary.Split` (`self.Name`) "-"))
  (set `self.MazeCenter` (`Actor.K2_GetActorLocation` (`self.Maze`)))
  (set `self.Sector` (`KismetStringLibrary.Conv_StringToInt` _lefts))
  (set `self.Level` (`KismetStringLibrary.Conv_StringToInt` _rights))
  (`self.CalculateCornerLocation` ForwardVector NumSector InnerRadius RingDistance)
  (return))